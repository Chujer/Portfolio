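; Self-running blue dragon attack actor that plays the Att3 animation at double speed with water effects, then dissolves and destroys itself.
; BeginPlay spawns a portal, an attached water trail and, when FTrue is set, a ground tornado plus a delayed impact.
; A timed timeline drives the "amount" parameter on swapped-in dissolve materials for mesh and tail, while the trail shuts off and eye and Niagara effects hide before destruction.
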(event `self.ReceiveBeginPlay`
  (bind _portal (`self.Portal`))
  (bind _skeletalmesh (`self.SkeletalMesh`))
  (bind _skeletalmesh_2 (`self.SkeletalMesh`))
  (`SkeletalMeshComponent.PlayAnimation` _skeletalmesh "/Game/DragonAbility/Anim/Att3.Att3" false)
  (`SkeletalMeshComponent.SetPlayRate` _skeletalmesh 2.0)
  (`|ExecutionSequence`
    (:`then_0`
      (`KismetSystemLibrary.Delay` 1.8)
      (`|ExecutionSequence`
        (:`then_0`
          (`PrimitiveComponent.SetMaterial` _skeletalmesh_2 0 "/Game/DragonAbility/Mat_IN/M_BlueDiss_IN.M_BlueDiss_IN")
          (bind (_direction _dis) (`Timeline|Dissolve` :!label _label)
            (:`Update`
              (`MeshComponent.SetScalarParameterValueOnMaterials` (`self.SkeletalMesh`) "amount" _dis)
              (`MeshComponent.SetScalarParameterValueOnMaterials` (`self.Tail`) "amount" _dis))))
        (:`then_1`
          (`PrimitiveComponent.SetMaterial` _skeletalmesh_2 1 "/Game/DragonAbility/Mat_IN/M_BlueDiss_IN.M_BlueDiss_IN")
          (goto _label))
        (:`then_2`
          (`PrimitiveComponent.SetMaterial` _skeletalmesh_2 2 "/Game/DragonAbility/Mat_IN/M_BlueDiss_IN.M_BlueDiss_IN")
          (goto _label))
        (:`then_3`
          (`PrimitiveComponent.SetMaterial` (`self.Tail`) 0 "/Game/DragonAbility/Mat_IN/M_BlueDiss_IN.M_BlueDiss_IN")
          (goto _label))))
    (:`then_1`
      (bind _returnvalue (`GameplayStatics.SpawnEmitterAttached` "/Game/DragonAbility/FX/PS/Water/P_WaterTrail.P_WaterTrail" (`self.SkeletalMesh`) "0" (0.0 0.0 0.0) (struct) (1.0 1.0 1.0) "SnapToTargetIncludingScale"))
      (set `ParticleSystemComponent.InstanceParameters` (`|MakeArray` (make `ParticleSysParam` "VertSurfaceActor" "PSPT_Actor" 0.0 0.0 (0.0 0.0 0.0) (0.0 0.0 0.0) (struct) self)) _returnvalue)
      (`KismetSystemLibrary.Delay` 1.8)
      (`ActorComponent.Deactivate` _returnvalue)
      (`|ExecutionSequence`
        (:`then_0`
          (`KismetSystemLibrary.Delay` 1.0)
          (`self.K2_DestroyActor`))
        (:`then_1`
          (`SceneComponent.SetVisibility` (`self.SM_EyeFX`) false false)
          (`SceneComponent.SetVisibility` (`self.Niagara1`) false false)
          (`SceneComponent.SetVisibility` (`self.Niagara`) false false))))
    (:`then_2`
      (`KismetSystemLibrary.Delay` 1.4)
      (if (`self.FTrue`)
        (`GameplayStatics.SpawnEmitterAtLocation` "/Game/DragonAbility/FX/PS/Water/P_WaterIpact.P_WaterIpact" (`SceneComponent.K2_GetComponentLocation` (`self.ImpactGround`)))))
    (:`then_3`
      (if (`self.FTrue`)
        (`NiagaraFunctionLibrary.SpawnSystemAtLocation` "/Game/DragonAbility/FX/NS/Water/Ns_WaterTornado.Ns_WaterTornado" (`SceneComponent.K2_GetComponentLocation` (`self.ImpactGround`)))))
    (:`then_4`
      (`GameplayStatics.SpawnEmitterAtLocation` "/Game/DragonAbility/FX/PS/P_Portal.P_Portal" (+ (`SceneComponent.K2_GetComponentLocation` _portal) (`self.GetActorForwardVector`)) (`SceneComponent.K2_GetComponentRotation` _portal)))))

(fn `UserConstructionScript`)