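; Player character Blueprint for third-person combat with sword, bow and spear, skills, lock-on targeting and camera zoom.
; Input events gate on StateComponent and delegate to Weapon, Moving and Target components, with high horizontal speed turning attacks into dash attacks.
; BeginPlay sets pitch limits and creates crosshair and hold-to-show menu widgets.
; Tick interpolates spring-arm zoom outside bow mode and displays action mode; landing feeds ParkourComponent, whose input trigger is unwired.
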(event `self.ReceiveBeginPlay`
  (`|ExecutionSequence`
    (:`then_0`
      (`/Game/Components/MovingComponent.DisableControlRotation` (`self.MovingComponent`)))
    (:`then_1`
      (bind _asplayer_controller (cast `PlayerController` (`self.GetController`)))
      (bind _playercameramanager (`PlayerController.PlayerCameraManager` _asplayer_controller))
      (set `PlayerCameraManager.ViewPitchMin` -25.0 _playercameramanager)
      (set `PlayerCameraManager.ViewPitchMax` 40.0 _playercameramanager))
    (:`then_2`
      (set `self.Zooming` (`SpringArmComponent.TargetArmLength` (`self.SpringArm`))))
    (:`then_3`
      (bind _returnvalue (`|CreateWidget` "/Game/Widgets/WB_Menu.WB_Menu_C"))
      (bind _output_get (set `self.Menu` _returnvalue))
      (`UserWidget.AddToViewport` _output_get 0)
      (`Widget.SetVisibility` _output_get "Hidden"))
    (:`then_4`
      (bind _asplayer_controller_2 (cast `PlayerController` (`self.GetController`)))
      (bind _returnvalue_2 (`|CreateWidget` "/Game/Widgets/WB_Crosshair.WB_Crosshair_C" _asplayer_controller_2))
      (`UserWidget.AddToViewport` _returnvalue_2 0))))

(event `InputAxis|MoveForward`
  (params (AxisValue :type "Float (single-precision)"))
  (bind (_returnvalue_roll _returnvalue_pitch _returnvalue_yaw) (`KismetMathLibrary.BreakRotator` (`self.GetControlRotation`)))
  (if (`/Game/Components/MovingComponent.IsCanMove` (`self.MovingComponent`))
    (if (not (> AxisValue 0.0))
      (set `CharacterMovementComponent.MaxWalkSpeed` 600.0 (`self.CharacterMovement`)))
    (`self.AddMovementInput` (`KismetMathLibrary.GetForwardVector` (`KismetMathLibrary.MakeRotator` 0.0 0.0 _returnvalue_yaw)) AxisValue)))

(event `InputAxis|MoveRight`
  (params (AxisValue :type "Float (single-precision)"))
  (bind (_returnvalue_roll _returnvalue_pitch _returnvalue_yaw) (`KismetMathLibrary.BreakRotator` (`self.GetControlRotation`)))
  (if (`/Game/Components/MovingComponent.IsCanMove` (`self.MovingComponent`))
    (`self.AddMovementInput` (`KismetMathLibrary.GetRightVector` (`KismetMathLibrary.MakeRotator` 0.0 0.0 _returnvalue_yaw)) AxisValue)))

(event `InputAction|Sprint`
  (params (Key :type "Key Structure"))
  (bind _charactermovement (`self.CharacterMovement`))
  (:`Pressed`
    (set `CharacterMovementComponent.MaxWalkSpeed` 1000.0 _charactermovement)
    (set `self.IsSprint` true))
  (:`Released`
    (set `CharacterMovementComponent.MaxWalkSpeed` 600.0 _charactermovement)
    (set `self.IsSprint` false)))

(event `InputAxis|HorizontalLook`
  (params (AxisValue :type "Float (single-precision)"))
  (if (not (`/Game/Components/MovingComponent.IsFixedCamera` (`self.MovingComponent`)))
    (`self.AddControllerYawInput` AxisValue)))

(event `InputAxis|VerticalLook`
  (params (AxisValue :type "Float (single-precision)"))
  (if (not (`/Game/Components/MovingComponent.IsFixedCamera` (`self.MovingComponent`)))
    (`self.AddControllerPitchInput` AxisValue)))

(event `InputAction|Sword`
  (params (Key :type "Key Structure"))
  (:`Pressed`
    (if (`/Game/Components/StateComponent.IsIdleMode` (`self.StateComponent`))
      (`/Game/Components/WeaponComponent.SetSwordMode` (`self.WeaponComponent`)))))

(event `InputAction|Action`
  (params (Key :type "Key Structure"))
  (:`Pressed`
    (if (> (`KismetMathLibrary.VSizeXY` (`self.GetVelocity`)) 700.0)
      (`/Game/Components/StateComponent.SetLeftActionMode` (`self.StateComponent`))
      (`/Game/Components/WeaponComponent.DashLeftAction` (`self.WeaponComponent`))
      (elif (and (`|EnumInequality` (`/Game/Components/StateComponent.GetActionMode` (`self.StateComponent`)) "NewEnumerator2") (`/Game/Components/StateComponent.IsIdleMode` (`self.StateComponent`)))
        (`/Game/Components/StateComponent.SetLeftActionMode` (`self.StateComponent`))
        (`/Game/Components/WeaponComponent.DoAction` (`self.WeaponComponent`))
        (else
          (`/Game/Components/WeaponComponent.DoAction` (`self.WeaponComponent`)))))))

(event `InputAction|Bow`
  (params (Key :type "Key Structure"))
  (:`Pressed`
    (if (`/Game/Components/StateComponent.IsIdleMode` (`self.StateComponent`))
      (`/Game/Components/WeaponComponent.SetBowMode` (`self.WeaponComponent`)))))

(event `InputAction|SubAction`
  (params (Key :type "Key Structure"))
  (bind _weaponcomponent (`self.WeaponComponent`))
  (:`Pressed`
    (if (`self.IsNotBowMode`)
      (if (and (`|EnumInequality` (`/Game/Components/StateComponent.GetActionMode` (`self.StateComponent`)) "NewEnumerator2") (`/Game/Components/StateComponent.IsIdleMode` (`self.StateComponent`)))
        (if (> (`KismetMathLibrary.VSizeXY` (`self.GetVelocity`)) 700.0)
          (`/Game/Components/StateComponent.SetLeftActionMode` (`self.StateComponent`))
          (`/Game/Components/WeaponComponent.DashRightAction` (`self.WeaponComponent`))
          (else
            (`/Game/Components/StateComponent.SetRightActionMode` (`self.StateComponent`))
            (`/Game/Components/WeaponComponent.DoAction` (`self.WeaponComponent`))))
        (else
          (`/Game/Components/WeaponComponent.DoAction` (`self.WeaponComponent`))))
      (else
        (`/Game/Components/WeaponComponent.Pressed` _weaponcomponent))))
  (:`Released`
    (`/Game/Components/WeaponComponent.Released` _weaponcomponent)))

(event `InputAction|UpperSkill`
  (params (Key :type "Key Structure"))
  (:`Pressed`
    (if (`/Game/Components/StateComponent.IsIdleMode` (`self.StateComponent`))
      (`/Game/Components/StateComponent.SetLeftActionMode` (`self.StateComponent`))
      (`/Game/Components/WeaponComponent.Do_Upper_Action` (`self.WeaponComponent`)))))

(event `InputAction|Skill_1`
  (params (Key :type "Key Structure"))
  (:`Pressed`
    (if (`/Game/Components/StateComponent.IsIdleMode` (`self.StateComponent`))
      (`/Game/Components/StateComponent.SetSkillMode` (`self.StateComponent`))
      (`/Game/Components/WeaponComponent.Do_Skill_Pressed` (`self.WeaponComponent`) 0)))
  (:`Released`
    (`/Game/Components/WeaponComponent.Do_Released` (`self.WeaponComponent`))))

(event `InputAction|Skill_2`
  (params (Key :type "Key Structure"))
  (:`Pressed`
    (if (`/Game/Components/StateComponent.IsIdleMode` (`self.StateComponent`))
      (`/Game/Components/StateComponent.SetSkillMode` (`self.StateComponent`))
      (`/Game/Components/WeaponComponent.Do_Skill_Pressed` (`self.WeaponComponent`) 1)))
  (:`Released`
    (`/Game/Components/WeaponComponent.Do_Released` (`self.WeaponComponent`))))

(event `InputAction|Skill_3`
  (params (Key :type "Key Structure"))
  (:`Pressed`
    (if (`/Game/Components/StateComponent.IsIdleMode` (`self.StateComponent`))
      (`/Game/Components/StateComponent.SetSkillMode` (`self.StateComponent`))
      (`/Game/Components/WeaponComponent.Do_Skill_Pressed` (`self.WeaponComponent`) 2)))
  (:`Released`
    (`/Game/Components/WeaponComponent.Do_Released` (`self.WeaponComponent`))))

(event `InputAction|Skill_4`
  (params (Key :type "Key Structure"))
  (:`Pressed`
    (if (`/Game/Components/StateComponent.IsIdleMode` (`self.StateComponent`))
      (`/Game/Components/StateComponent.SetSkillMode` (`self.StateComponent`))
      (`/Game/Components/WeaponComponent.Do_Skill_Pressed` (`self.WeaponComponent`) 3)))
  (:`Released`
    (`/Game/Components/WeaponComponent.Do_Released` (`self.WeaponComponent`))))

(event `InputAction|Dash`
  (params (Key :type "Key Structure"))
  (:`Pressed`
    (if (not (`/Game/Components/WeaponComponent.IsUnamredMode` (`self.WeaponComponent`)))
      (`self.PlayAnimMontage` "/Game/Character/Montages/Katana/Dash/DeshReady.DeshReady"))))

(event `InputAction|Spear`
  (params (Key :type "Key Structure"))
  (:`Pressed`
    (if (`/Game/Components/StateComponent.IsIdleMode` (`self.StateComponent`))
      (`/Game/Components/WeaponComponent.SetSpearMode` (`self.WeaponComponent`)))))

(event `self.ReceiveTick`
  (params (DeltaSeconds :type "Float (single-precision)"))
  (`self.Apply_Zoom`)
  (`self.SetText` (`KismetTextLibrary.Conv_StringToText` (`|GetEnumeratorNameAsString` (`/Game/Components/StateComponent.GetActionMode` (`self.StateComponent`)))))
  (`TextRenderComponent.K2_SetText` (`self.TextRender`) (`self.Text`)))

(event `Apply_Zoom`
  (bind _zooming (`self.Zooming`))
  (bind (_zoomdata_speed _zoomdata_minrange _zoomdata_maxrange _zoomdata_interpspeed) (break `/Game/Player/FZoomData` (`self.ZoomData`)))
  (bind _targetarmlength (`SpringArmComponent.TargetArmLength` (`self.SpringArm`)))
  (if (and (`self.IsNotBowMode`) (not (`KismetMathLibrary.NearlyEqual_FloatFloat` _targetarmlength _zooming 0.1)))
    (set `SpringArmComponent.TargetArmLength` (`KismetMathLibrary.FInterpTo` _targetarmlength _zooming (`GameplayStatics.GetWorldDeltaSeconds`) _zoomdata_interpspeed) (`self.SpringArm`))))

(event `InputAxis|Zoom`
  (params (AxisValue :type "Float (single-precision)"))
  (bind (_zoomdata_speed _zoomdata_minrange _zoomdata_maxrange) (break `/Game/Player/FZoomData` (`self.ZoomData`)))
  (if (`self.IsNotBowMode`)
    (set `self.Zooming` (`KismetMathLibrary.FClamp` (+ (`self.Zooming`) (* AxisValue _zoomdata_speed)) _zoomdata_minrange _zoomdata_maxrange))))

(event `InputAction|Targeting`
  (params (Key :type "Key Structure"))
  (:`Pressed`
    (`/Game/Components/TargetComponent.Toggle_Target` (`self.TargetComponent`))))

(event `self.OnLanded`
  (params (Hit :type "HitResult Structure (by ref)"))
  ;[1 1 1] 플레이어 착지
  (if (`|EnumEquality` (`/Game/Components/StateComponent.GetActionMode` (`self.StateComponent`)) "NewEnumerator2")
    (`/Game/Components/StateComponent.SetLeftActionMode` (`self.StateComponent`))
    (else
      (`/Game/Parkour/ParkourComponent.DoFarkour_LandMode` (`self.ParkourComponent`)))))

(event `InputAction|Menu`
  (params (Key :type "Key Structure"))
  (bind _returnvalue (`GameplayStatics.GetPlayerController` 0))
  (bind _returnvalue_2 (`GameplayStatics.GetPlayerController` 0))
  (:`Pressed`
    (if (`/Game/Components/StateComponent.IsIdleMode` (`self.StateComponent`))
      (`Widget.SetVisibility` (`self.Menu`) "Visible")
      (set `PlayerController.bShowMouseCursor` true _returnvalue_2)
      (`WidgetBlueprintLibrary.SetInputMode_GameAndUIEx` _returnvalue_2 null)))
  (:`Released`
    (`Widget.SetVisibility` (`self.Menu`) "Hidden" :!label _label)
    (set `PlayerController.bShowMouseCursor` false _returnvalue)
    (`WidgetBlueprintLibrary.SetInputMode_GameOnly` _returnvalue)))

(event `Menu_Hide`
  (goto _label))

(fn `EndNiagaraEffect`
  (bind _niagara (`self.Niagara`))
  (`/Engine/EditorBlueprintResources/StandardMacros.IsValid` _niagara
    (:`Is Valid`
      (`SceneComponent.SetVisibility` _niagara false false))))

(fn `IsNotBowMode`
  (returns (ReturnValue :type Boolean))
  (return (not (`/Game/Components/WeaponComponent.IsBowMode` (`self.WeaponComponent`)))))

(fn `SetNiagaraEffect`
  (params (Niagara :type "NiagaraSystem Object Reference") (Location :type "Vector Structure") (Rotation :type "Rotator Structure") (Scale :type "Vector Structure"))
  (`NiagaraFunctionLibrary.SpawnSystemAtLocation` Niagara Location Rotation Scale))

(fn `SetRootNiagaraEffect`
  (params (Niagara :type "NiagaraSystem Object Reference"))
  (bind _returnvalue (`NiagaraFunctionLibrary.SpawnSystemAttached` Niagara (`self.Mesh`) "Root" (0.0 0.0 0.0) (struct) "KeepRelativeOffset"))
  (set `self.Niagara` _returnvalue)
  (add `self.EndNotify` (`|CreateDelegate` :!event `EndNiagaraEffect`)))

(fn `SetText`
  (params (Text :type Text))
  (set `self.Text` Text))

(fn `UserConstructionScript`)