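; Enemy character that takes hits, reacts and dies, with launch and zero-gravity support for player air combos.
; Damaged stores HitData and enters Hitted state, routing to normal or in-air knockdown reactions after subtracting health; DashDamaged reacts without health loss.
; Reactions combine facing the attacker, montage, red material flash, launches, effects and camera shake.
; Hit stop nearly freezes movable-mesh actors through CustomTimeDilation, restored by timer.
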(event `self.ReceiveBeginPlay`
  (for _array_element (`MeshComponent.GetMaterials` (`self.Mesh`))
    (bind _returnvalue (`KismetMaterialLibrary.CreateDynamicMaterialInstance` _array_element))
    (bind _returnvalue_2 (`KismetArrayLibrary.Array_Add` (`self.Materials`) _returnvalue))
    (`PrimitiveComponent.SetMaterial` (`self.Mesh`) _returnvalue_2 _returnvalue))
  (set `self.Health` (`self.MaxHealth`))
  (add `/Game/Components/StateComponent.OnStateTypeChanged` (`self.StateComponent`) (`|CreateDelegate` :!event `OnStateTypeChanged`)))

(event `OnStateTypeChanged`
  (params (InPrevType :type "/Game/Components/EStateType Enum" :default "NewEnumerator0") (InNewType :type "/Game/Components/EStateType Enum" :default "NewEnumerator0"))
  (bind (_hitdata_damage _hitdata_montage _hitdata_playrate _hitdata_canmove _hitdata_launch _hitdata_hitstop _hitdata_sound _hitdata_shakeclass _hitdata_effect _hitdata_effectlocation _hitdata_effectscale _hitdata_uplaunch) (break `/Game/Weapons/FHitData` (`self.HitData`)))
  (switch `/Game/Components/EStateType` InNewType
    (:`NewEnumerator4`
      (if (and (`NavMovementComponent.IsFalling` (`self.CharacterMovement`)) (not (`/Game/Components/GravityComponent.IsZeroGravity` (`self.GravityComponent`))) (not (`/Game/Components/GravityComponent.IsZeroGravity` (`self.GetComponentByClass` (`self.Attacker`) "/Game/Components/GravityComponent.GravityComponent_C"))) (not (> _hitdata_uplaunch 0.0)))
        (`self.InAirHitted`)
        (else
          (`self.Hitted`))))))

(event `InAirHitted`
  (bind _returnvalue (`self.K2_GetActorRotation`))
  (bind (_hitdata_damage _hitdata_montage _hitdata_playrate _hitdata_canmove _hitdata_launch _hitdata_hitstop _hitdata_sound _hitdata_shakeclass _hitdata_effect _hitdata_effectlocation _hitdata_effectscale) (break `/Game/Weapons/FHitData` (`self.HitData`)))
  (bind (_hitdata_damage_2 _hitdata_montage_2 _hitdata_playrate_2 _hitdata_canmove_2 _hitdata_launch_2 _hitdata_hitstop_2) (break `/Game/Weapons/FHitData` (`self.HitData`)))
  (bind (_hitdata_damage_3 _hitdata_montage_3 _hitdata_playrate_3 _hitdata_canmove_3 _hitdata_launch_3 _hitdata_hitstop_3) (break `/Game/Weapons/FHitData` (`self.HitData`)))
  (bind (_damage _montage _playrate _canmove _launch _hitstop _sound _shakeclass) (break `/Game/Weapons/FHitData` (`self.HitData`)))
  (bind (_returnvalue_roll _returnvalue_pitch _returnvalue_yaw) (`KismetMathLibrary.BreakRotator` (`KismetMathLibrary.FindLookAtRotation` (`self.K2_GetActorLocation`) (`self.K2_GetActorLocation` (`self.Attacker`)))))
  (bind (_returnvalue_x _returnvalue_y) (`KismetMathLibrary.BreakVector` (* (`self.GetActorForwardVector` (`self.Attacker`)) (`.Launch_14_81E2FC3C40CD275BC7E7E48C31968CB2` (break `/Game/Weapons/FHitData` (`self.HitData`))))))
  (bind (_returnvalue_x_2 _returnvalue_y_2) (`KismetMathLibrary.BreakVector` (* (`self.GetActorForwardVector` (`self.Attacker`)) (`.Launch_14_81E2FC3C40CD275BC7E7E48C31968CB2` (break `/Game/Weapons/FHitData` (`self.HitData`))))))
  ;[1 1 1] 지상 공중 데미지
  (bind _output_get (set `self.Health` (`KismetMathLibrary.FClamp` (- (`self.Health`) (`.Damage_2_3B991AA742D83F1BDBECA8BAC3E986B1` (break `/Game/Weapons/FHitData` (`self.HitData`)))) 0.0 (`self.MaxHealth`))))
  (if (<= _output_get 0.0)
    (`self.Dead`)
    (else
      (`self.K2_SetActorRotation` (`KismetMathLibrary.MakeRotator` 0.0 0.0 _returnvalue_yaw))
      (`self.PlayAnimMontage` "/Game/Character/Montages/Common/KNockDown1_Test_Montage.KNockDown1_Test_Montage")
      (`|ExecutionSequence`
        (:`then_0`
          (for _array_element (`self.Materials`)
            (`MaterialInstanceDynamic.SetVectorParameterValue` _array_element "BodyColor" (struct :`R` 1.0 :`A` 1.0)))
          (`KismetSystemLibrary.Delay` 0.15)
          (for _array_element_2 (`self.Materials`)
            (`MaterialInstanceDynamic.SetVectorParameterValue` _array_element_2 "BodyColor" (struct :`R` 1.0 :`G` 1.0 :`B` 1.0 :`A` 1.0)))
          (if (`.WithLuanch_38_C05894F34CAD19FF59B2D0870A089DF9` (break `/Game/Weapons/FHitData` (`self.HitData`)))
            (set `MovementComponent.Velocity` (0.0 0.0 0.0) (`self.CharacterMovement`))
            (`self.LaunchCharacter` (* (`KismetMathLibrary.MakeVector` _returnvalue_x _returnvalue_y 250.0) 0.5) true true)
            (`self.LaunchCharacter` (`self.Attacker`) (* (`self.GetActorForwardVector` (`self.Attacker`)) (`.Launch_14_81E2FC3C40CD275BC7E7E48C31968CB2` (break `/Game/Weapons/FHitData` (`self.HitData`)))) true false)
            (else
              (`self.LaunchCharacter` (`KismetMathLibrary.MakeVector` _returnvalue_x_2 _returnvalue_y_2 150.0) false true))))
        (:`then_1`
          (`GameplayStatics.SpawnEmitterAtLocation` _hitdata_effect (+ (`self.K2_GetActorLocation`) (`KismetMathLibrary.GreaterGreater_VectorRotator` _hitdata_effectlocation _returnvalue)) _returnvalue _hitdata_effectscale)
          (`GameplayStatics.SpawnSoundAtLocation` (`.Sound_19_A56468664F7CF95069D4878B8776BFE3` (break `/Game/Weapons/FHitData` (`self.HitData`))) (`self.K2_GetActorLocation`) (struct) 1.0 1.0 0.0 null null)
          (if (`KismetSystemLibrary.IsValidClass` _shakeclass)
            (`PlayerCameraManager.StartCameraShake` :`self` (`GameplayStatics.GetPlayerCameraManager` 0) :`ShakeClass` _shakeclass))
          (if (not (`KismetMathLibrary.NearlyEqual_FloatFloat` _hitdata_hitstop_2 0.0 1e-05))
            (bind _outactors (`GameplayStatics.GetAllActorsOfClass` "/Script/Engine.Actor"))
            (for _array_element_3 _outactors
              (bind _returnvalue_2 (`self.GetComponentByClass` _array_element_3 "/Script/Engine.MeshComponent"))
              (`/Engine/EditorBlueprintResources/StandardMacros.IsValid` _returnvalue_2
                (:`Is Valid`
                  (if (`|EnumEquality` (`SceneComponent.Mobility` _returnvalue_2) "Movable")
                    (`KismetArrayLibrary.Array_Add` (`self.DelationActors`) _array_element_3)
                    (set `Actor.CustomTimeDilation` 0.001 _array_element_3)))))
            (`KismetSystemLibrary.K2_SetTimer` self "RestoreTimeDelation2" _hitdata_hitstop_3)
            (`self.PlayHitStop_Exit2`)))))))

(event `PlayHitStop_Exit2`
  ;[1 1 1] 지상 공중 데미지
)

(event `RestoreTimeDelation2`
  (bind _delationactors (`self.DelationActors`))
  ;[1 1 1] 지상 공중 데미지
  (for _array_element _delationactors
    (set `Actor.CustomTimeDilation` 1.0 _array_element))
  (`KismetArrayLibrary.Array_Clear` _delationactors))

(event `Hitted`
  (bind _returnvalue (`self.K2_GetActorRotation`))
  (bind (_returnvalue_x _returnvalue_y _returnvalue_z) (`KismetMathLibrary.BreakVector` (`self.K2_GetActorLocation`)))
  (bind (_hitdata_damage _hitdata_montage _hitdata_playrate _hitdata_canmove _hitdata_launch _hitdata_hitstop _hitdata_sound _hitdata_shakeclass _hitdata_effect _hitdata_effectlocation _hitdata_effectscale) (break `/Game/Weapons/FHitData` (`self.HitData`)))
  (bind (_hitdata_damage_2 _hitdata_montage_2 _hitdata_playrate_2 _hitdata_canmove_2 _hitdata_launch_2 _hitdata_hitstop_2) (break `/Game/Weapons/FHitData` (`self.HitData`)))
  (bind (_hitdata_damage_3 _hitdata_montage_3 _hitdata_playrate_3 _hitdata_canmove_3 _hitdata_launch_3 _hitdata_hitstop_3) (break `/Game/Weapons/FHitData` (`self.HitData`)))
  (bind (_damage _montage _playrate) (break `/Game/Weapons/FHitData` (`self.HitData`)))
  (bind (_damage_2 _montage_2 _playrate_2 _canmove _launch _hitstop _sound _shakeclass _effect _effectlocation _effectscale _uplaunch) (break `/Game/Weapons/FHitData` (`self.HitData`)))
  (bind (_damage_3 _montage_3 _playrate_3 _canmove_2 _launch_2 _hitstop_2 _sound_2 _shakeclass_2 _effect_2 _effectlocation_2 _effectscale_2 _uplaunch_2) (break `/Game/Weapons/FHitData` (`self.HitData`)))
  (bind (_damage_4 _montage_4 _playrate_4 _canmove_3 _launch_3) (break `/Game/Weapons/FHitData` (`self.HitData`)))
  (bind (_damage_5 _montage_5 _playrate_5 _canmove_4 _launch_4 _hitstop_3 _sound_3 _shakeclass_3 _effect_3 _effectlocation_3 _effectscale_3 _uplaunch_3) (break `/Game/Weapons/FHitData` (`self.HitData`)))
  (bind (_damage_6 _montage_6 _playrate_6 _canmove_5 _launch_5 _hitstop_4 _sound_4 _shakeclass_4) (break `/Game/Weapons/FHitData` (`self.HitData`)))
  (bind (_returnvalue_x_2 _returnvalue_y_2 _returnvalue_z_2) (`KismetMathLibrary.BreakVector` (`self.K2_GetActorLocation` (`self.Attacker`))))
  (bind (_returnvalue_roll _returnvalue_pitch _returnvalue_yaw) (`KismetMathLibrary.BreakRotator` (`KismetMathLibrary.FindLookAtRotation` (`self.K2_GetActorLocation`) (`self.K2_GetActorLocation` (`self.Attacker`)))))
  (bind (_returnvalue_x_3 _returnvalue_y_3) (`KismetMathLibrary.BreakVector` (* (`self.GetActorForwardVector` (`self.Attacker`)) _launch)))
  (bind (_returnvalue_x_4 _returnvalue_y_4) (`KismetMathLibrary.BreakVector` (* (`self.GetActorForwardVector` (`self.Attacker`)) _launch_2)))
  (bind _returnvalue_2 (* (`self.GetActorForwardVector` (`self.Attacker`)) (`.Launch_14_81E2FC3C40CD275BC7E7E48C31968CB2` (break `/Game/Weapons/FHitData` (`self.HitData`)))))
  (bind _returnvalue_x_5 (`KismetMathLibrary.BreakVector` (* (`self.GetActorForwardVector` (`self.Attacker`)) _launch_3)))
  (bind (_returnvalue_x_6 _returnvalue_y_5) (`KismetMathLibrary.BreakVector` (* (`self.GetActorForwardVector` (`self.Attacker`)) _launch_4)))
  (bind (_returnvalue_x_7 _returnvalue_y_6 _returnvalue_z_3) (`KismetMathLibrary.BreakVector` (`KismetMathLibrary.MakeVector` _returnvalue_x_6 _returnvalue_y_5 _uplaunch_3)))
  (bind _output_get (set `self.Health` (`KismetMathLibrary.FClamp` (- (`self.Health`) (`.Damage_2_3B991AA742D83F1BDBECA8BAC3E986B1` (break `/Game/Weapons/FHitData` (`self.HitData`)))) 0.0 (`self.MaxHealth`))))
  (if (<= _output_get 0.0)
    (`self.Dead`)
    (else
      (`self.K2_SetActorRotation` (`KismetMathLibrary.MakeRotator` 0.0 0.0 _returnvalue_yaw))
      (if (`KismetStringLibrary.EqualEqual_StrStr` (`KismetSystemLibrary.GetPathName` (`.Montage_5_481175224EDAB3DD368922BBF744F911` (break `/Game/Weapons/FHitData` (`self.HitData`)))))
        (`self.PlayAnimMontage` (`KismetArrayLibrary.Array_Random` (`self.NomalHitMontage`)) (`.PlayRate_8_683D35604E98ACE7C8B3F587A35685F6` (break `/Game/Weapons/FHitData` (`self.HitData`))))
        (else
          (`self.PlayAnimMontage` _montage _playrate)))
      (`|ExecutionSequence`
        (:`then_0`
          (for _array_element (`self.Materials`)
            (`MaterialInstanceDynamic.SetVectorParameterValue` _array_element "BodyColor" (struct :`R` 1.0 :`A` 1.0)))
          (`KismetSystemLibrary.Delay` 0.15)
          (for _array_element_2 (`self.Materials`)
            (`MaterialInstanceDynamic.SetVectorParameterValue` _array_element_2 "BodyColor" (struct :`R` 1.0 :`G` 1.0 :`B` 1.0 :`A` 1.0)))
          (if (`/Game/Components/GravityComponent.IsZeroGravity` (`self.GravityComponent`))
            (`/Game/Components/GravityComponent.StartZeroGravity` (`self.GravityComponent`))
            (`KismetSystemLibrary.K2_SetTimerDelegate` (delegate `End Zero Gravity`) 0.8))
          (if (> (`.UpLaunch_42_8E9CD972491CE58250AF0885C99147A6` (break `/Game/Weapons/FHitData` (`self.HitData`))) 0.0)
            (cast `/Game/Player/BP_Player` (`self.Attacker`))
            (set `MovementComponent.Velocity` (0.0 0.0 0.0) (`self.CharacterMovement`))
            (`self.LaunchCharacter` (`KismetMathLibrary.MakeVector` _returnvalue_x_4 _returnvalue_y_4 (- _uplaunch_2 (- _returnvalue_z _returnvalue_z_2))) true)
            (if (`.WithLuanch_38_C05894F34CAD19FF59B2D0870A089DF9` (break `/Game/Weapons/FHitData` (`self.HitData`)))
              (`self.LaunchCharacter` (`self.Attacker`) (`KismetMathLibrary.MakeVector` _returnvalue_x_3 _returnvalue_y_3 _uplaunch) false true)
              (`KismetSystemLibrary.K2_SetTimer` (`self.GetComponentByClass` (`self.Attacker`) "/Game/Components/StateComponent.StateComponent_C") "SetAirComboMode" 0.1))
            (elif (`.WithLuanch_38_C05894F34CAD19FF59B2D0870A089DF9` (break `/Game/Weapons/FHitData` (`self.HitData`)))
              (`self.LaunchCharacter` _returnvalue_2 true true)
              (`self.LaunchCharacter` (`self.Attacker`) _returnvalue_2 true false)
              (bind _asbp_player (cast `/Game/Player/BP_Player` (`self.Attacker`)))
              (if (`/Game/Components/StateComponent.IsWithAirComboMode` (`/Game/Player/BP_Player.StateComponent` _asbp_player))
                (`/Game/Components/GravityComponent.StartZeroGravity` (`self.GravityComponent`))
                (`KismetSystemLibrary.K2_SetTimerDelegate` (`|CreateDelegate` :!event `End Zero Gravity`) 0.8))
              (elif (`/Game/Components/StateComponent.IsWithAirComboMode` (`self.GetComponentByClass` (`self.Attacker`) "/Game/Components/StateComponent.StateComponent_C"))
                (`self.LaunchCharacter` (`KismetMathLibrary.MakeVector` _returnvalue_x_5 0.0 (* _launch_3 -10.0)))
                (`/Game/Components/GravityComponent.EndZeroGravity` (`self.GravityComponent`))
                (`/Game/Components/GravityComponent.EndZeroGravity` (`self.GetComponentByClass` (`self.Attacker`) "/Game/Components/GravityComponent.GravityComponent_C"))
                (else
                  (`self.LaunchCharacter` (`KismetMathLibrary.MakeVector` _returnvalue_x_7 _returnvalue_y_6 _returnvalue_z_3) true))))))
        (:`then_1`
          (`GameplayStatics.SpawnEmitterAtLocation` _hitdata_effect (+ (`self.K2_GetActorLocation`) (`KismetMathLibrary.GreaterGreater_VectorRotator` _hitdata_effectlocation _returnvalue)) _returnvalue _hitdata_effectscale)
          (`GameplayStatics.SpawnSoundAtLocation` (`.Sound_19_A56468664F7CF95069D4878B8776BFE3` (break `/Game/Weapons/FHitData` (`self.HitData`))) (`self.K2_GetActorLocation`) (struct) 1.0 1.0 0.0 null null)
          (if (`KismetSystemLibrary.IsValidClass` _shakeclass_4)
            (`PlayerCameraManager.StartCameraShake` :`self` (`GameplayStatics.GetPlayerCameraManager` 0) :`ShakeClass` _shakeclass_4))
          (if (not (`KismetMathLibrary.NearlyEqual_FloatFloat` _hitdata_hitstop_2 0.0 1e-05))
            (bind _outactors (`GameplayStatics.GetAllActorsOfClass` "/Script/Engine.Actor"))
            (for _array_element_3 _outactors
              (bind _returnvalue_3 (`self.GetComponentByClass` _array_element_3 "/Script/Engine.MeshComponent"))
              (`/Engine/EditorBlueprintResources/StandardMacros.IsValid` _returnvalue_3
                (:`Is Valid`
                  (if (`|EnumEquality` (`SceneComponent.Mobility` _returnvalue_3) "Movable")
                    (`KismetArrayLibrary.Array_Add` (`self.DelationActors`) _array_element_3)
                    (set `Actor.CustomTimeDilation` 0.001 _array_element_3)))))
            (`KismetSystemLibrary.K2_SetTimer` self "RestoreTimeDelation" _hitdata_hitstop_3)
            (`self.PlayHitStop_Exit`)))))))

(event `PlayHitStop_Exit`)

(event `RestoreTimeDelation`
  (bind _delationactors (`self.DelationActors`))
  (for _array_element _delationactors
    (set `Actor.CustomTimeDilation` 1.0 _array_element))
  (`KismetArrayLibrary.Array_Clear` _delationactors))

(event `End Zero Gravity`
  (`/Game/Components/GravityComponent.EndZeroGravity` (`self.GravityComponent`)))

(event `DashHitted`
  (bind _returnvalue (`self.K2_GetActorRotation`))
  (bind (_hitdata_damage _hitdata_montage _hitdata_playrate _hitdata_canmove _hitdata_launch _hitdata_hitstop _hitdata_sound _hitdata_shakeclass _hitdata_effect _hitdata_effectlocation _hitdata_effectscale) (break `/Game/Weapons/FHitData` (`self.HitData`)))
  (bind (_damage _montage _playrate) (break `/Game/Weapons/FHitData` (`self.HitData`)))
  (bind (_returnvalue_roll _returnvalue_pitch _returnvalue_yaw) (`KismetMathLibrary.BreakRotator` (`KismetMathLibrary.FindLookAtRotation` (`self.K2_GetActorLocation`) (`self.K2_GetActorLocation` (`self.Attacker`)))))
  (`self.K2_SetActorRotation` (`KismetMathLibrary.MakeRotator` 0.0 0.0 _returnvalue_yaw))
  (`self.PlayAnimMontage` _montage _playrate)
  (`|ExecutionSequence`
    (:`then_0`
      (for _array_element (`self.Materials`)
        (`MaterialInstanceDynamic.SetVectorParameterValue` _array_element "BodyColor" (struct :`R` 1.0 :`A` 1.0)))
      (`KismetSystemLibrary.Delay` 0.15)
      (for _array_element_2 (`self.Materials`)
        (`MaterialInstanceDynamic.SetVectorParameterValue` _array_element_2 "BodyColor" (struct :`R` 1.0 :`G` 1.0 :`B` 1.0 :`A` 1.0)))
      (`GameplayStatics.SpawnEmitterAtLocation` _hitdata_effect (+ (`self.K2_GetActorLocation`) (`KismetMathLibrary.GreaterGreater_VectorRotator` _hitdata_effectlocation _returnvalue)) _returnvalue _hitdata_effectscale)
      (set `MovementComponent.Velocity` (0.0 0.0 0.0) (`self.CharacterMovement`))
      (cast `/Game/Player/BP_Player` (`self.Attacker`))
      (`self.LaunchCharacter` (`KismetMathLibrary.MakeVector` 0.0 0.0 (* (`.UpLaunch_42_8E9CD972491CE58250AF0885C99147A6` (break `/Game/Weapons/FHitData` (`self.HitData`))) 1.5)) true))
    (:`then_1`
      (`PlayerCameraManager.StartCameraShake` :`self` (`GameplayStatics.GetPlayerCameraManager` 0) :`ShakeClass` "/Game/Weapons/Sword/CS_SwordDash.CS_SwordDash_C")
      (bind _outactors (`GameplayStatics.GetAllActorsOfClass` "/Script/Engine.Actor"))
      (for _array_element_3 _outactors
        (bind _returnvalue_2 (`self.GetComponentByClass` _array_element_3 "/Script/Engine.MeshComponent"))
        (`/Engine/EditorBlueprintResources/StandardMacros.IsValid` _returnvalue_2
          (:`Is Valid`
            (if (`|EnumEquality` (`SceneComponent.Mobility` _returnvalue_2) "Movable")
              (`KismetArrayLibrary.Array_Add` (`self.DelationActors`) _array_element_3)
              (set `Actor.CustomTimeDilation` 0.001 _array_element_3)))))
      (`KismetSystemLibrary.K2_SetTimer` self "RestoreTimeDelation" 0.05)
      (`self.PlayHitStop_Exit`))))

(event `PlayHitStop_Exit_Dash`)

(event `RestoreTimeDelation_Dash`
  (bind _delationactors (`self.DelationActors`))
  (for _array_element _delationactors
    (set `Actor.CustomTimeDilation` 1.0 _array_element))
  (`KismetArrayLibrary.Array_Clear` _delationactors))

(event `/Game/IDamage.Damaged`
  (params (Attacker :type "Character Object Reference") (Causer :type "Actor Object Reference") (HitData :type "/Game/Weapons/FHitData Structure"))
  (set `self.Attacker` Attacker)
  (set `self.Causer` Causer)
  (set `self.HitData` HitData)
  (`/Game/Components/StateComponent.SetHittedMode` (`self.StateComponent`)))

(event `Dead`
  (`PrimitiveComponent.SetCollisionEnabled` (`self.CapsuleComponent`) "NoCollision")
  (`self.PlayAnimMontage` "/Game/Character/Montages/Enemy_DeadFall_Montage.Enemy_DeadFall_Montage"))

(event `End_Dead`
  (`self.K2_DestroyActor`))

(event `/Game/IDamage.DashDamaged`
  (params (Attacker :type "Character Object Reference") (Causer :type "Actor Object Reference") (HitData :type "/Game/Weapons/FHitData Structure"))
  (set `self.Attacker` Attacker)
  (set `self.Causer` Causer)
  (set `self.HitData` HitData)
  (`self.DashHitted`))

(event `self.OnLanded`
  (params (Hit :type "HitResult Structure (by ref)"))
  (if (`GameplayStatics.BreakHitResult` Hit)
    _))

(event `SetAnimDown`
  (params (DownDirection :type "Float (double-precision)"))
  (bind _asabp_character (cast `/Game/ABP_Character` (`SkeletalMeshComponent.GetAnimInstance` (`self.Mesh`))))
  (set `/Game/ABP_Character.IsDown` true _asabp_character)
  (set `/Game/ABP_Character.DownDirection` DownDirection _asabp_character))

(event `self.ReceiveTick`
  (params (DeltaSeconds :type "Float (single-precision)"))
  (`TextRenderComponent.K2_SetText` (`self.TextRender`) (`KismetTextLibrary.Conv_BoolToText` (`/Game/Components/GravityComponent.IsZeroGravity` (`self.GravityComponent`)))))

(fn `UserConstructionScript`)