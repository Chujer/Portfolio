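; GostActor is a ghost copy of a character, holding a snapshot of a skeletal pose until its owning BP_Player signals the end.
; Init copies the pose into a PoseableMesh, and BeginPlay attaches an added head mesh component at the Helmet socket and binds self-destruction to the player's EndNotify.
; SetMaterial applies dynamic instances of a given material to the body slots, reusing the created instance for the head.
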(event `Init`
  (params (SkeletalMesh :type "SkeletalMeshComponent Object Reference") (Weapon :type "/Game/Weapons/Weapon Object Reference"))
  (`/Engine/EditorBlueprintResources/StandardMacros.IsValid` SkeletalMesh
    (:`Is Valid`
      (`PoseableMeshComponent.CopyPoseFromSkeletalComponent` (`self.PoseableMesh`) SkeletalMesh)
      (set `self.Weapon` Weapon))))

(event `self.ReceiveBeginPlay`
  (bind _returnvalue (`AddComponent|NODE_AddSkeletalMeshComponent-0`))
  (bind _output_get (set `self.Head` _returnvalue))
  (`SceneComponent.K2_AttachToComponent` _output_get (`self.PoseableMesh`) "Helmet" "KeepRelative" "KeepRelative" "KeepRelative" true)
  (bind _asbp_player (cast `/Game/Player/BP_Player` (`self.GetOwner`)))
  (add `/Game/Player/BP_Player.EndNotify` _asbp_player (delegate `Destroy`)))

(event `Destroy`
  (`self.K2_DestroyActor`))

(event `SetMaterial`
  (params (NewParam :type "MaterialInstance Object Reference"))
  (`/Engine/EditorBlueprintResources/StandardMacros.IsValid` NewParam
    (:`Is Valid`
      (for (_ _array_index) (`MeshComponent.GetMaterials` (`self.PoseableMesh`))
        (bind _returnvalue (`KismetMaterialLibrary.CreateDynamicMaterialInstance` NewParam))
        (`PrimitiveComponent.SetMaterial` (`self.PoseableMesh`) _array_index _returnvalue))
      (for (_ _array_index_2) (`MeshComponent.GetMaterials` (`self.Head`))
        (`PrimitiveComponent.SetMaterial` (`self.Head`) _array_index_2 _returnvalue)))))

(fn `UserConstructionScript`)