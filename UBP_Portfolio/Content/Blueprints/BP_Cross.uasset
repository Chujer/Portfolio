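; BP_Cross is a debug visualizer for the cross product between a player's forward vector and the vector to an enemy.
; Each tick it draws arrows from the player for the to-enemy vector, the scaled forward vector and their cross product.
; It also prints the cross product, its dot with the player's up vector and that dot's sign, which indicates the enemy's left or right side.
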(event `self.ReceiveTick`
  (params (DeltaSeconds :type "Float (single-precision)"))
  (bind _returnvalue (`self.GetPlayerLocation`))
  (bind _returnvalue_2 (`self.GetPlayerLocation`))
  (bind _returnvalue_3 (`self.GetPlayerLocation`))
  (bind _player (`self.Player`))
  (bind _returnvalue_4 (`KismetMathLibrary.Cross_VectorVector` (`self.GetActorForwardVector` _player) (`self.GetPlayerToEnemy`)))
  (bind _returnvalue_5 (`KismetMathLibrary.Dot_VectorVector` _returnvalue_4 (`self.GetActorUpVector` _player)))
  (`|ExecutionSequence`
    (:`then_0`
      (`KismetSystemLibrary.DrawDebugArrow` _returnvalue_2 (+ _returnvalue_2 (`self.GetPlayerToEnemy`)) 100.0 (struct :`R` 1.0 :`A` 1.0)))
    (:`then_1`
      (`KismetSystemLibrary.DrawDebugArrow` _returnvalue (+ _returnvalue (* (`self.GetActorForwardVector` (`self.Player`)) 500.0)) 100.0 (struct :`G` 1.0 :`A` 1.0)))
    (:`then_2`
      (`KismetSystemLibrary.DrawDebugArrow` _returnvalue_3 (+ _returnvalue_3 _returnvalue_4) 100.0 (struct :`B` 1.0 :`A` 1.0))
      (`KismetSystemLibrary.PrintString` (`KismetStringLibrary.Concat_StrStr` (`KismetStringLibrary.Conv_VectorToString` _returnvalue_4) " / " (`KismetStringLibrary.Conv_DoubleToString` _returnvalue_5) " / " (`KismetStringLibrary.Conv_DoubleToString` (`KismetMathLibrary.SignOfFloat` _returnvalue_5)))))))

(fn `GetPlayerLocation`
  (returns (ReturnValue :type "Vector Structure"))
  (return (`self.K2_GetActorLocation` (`self.Player`))))

(fn `GetPlayerToEnemy`
  (returns (ReturnValue :type "Vector Structure"))
  (return (- (`self.K2_GetActorLocation` (`self.Enemy`)) (`self.GetPlayerLocation`))))

(fn `UserConstructionScript`)